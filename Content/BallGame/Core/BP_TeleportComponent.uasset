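; BP_TeleportComponent is a scene component that lets its owning actor teleport to an aimed point.
; On BeginPlay it spawns a BP_TeleportTarget marker.
; StartTeleporting shows the marker's sphere and enables a per-tick Visibility trace along the component's forward vector, moving the marker to blocking hits.
; EndTeleporting stops tracing and, if the last trace hit, moves the owner slightly above that point and hides the sphere.
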(event EventBeginPlay
  (Variables|Default|SetActorToBeTeleported (Components|GetOwner))
  (bind _returnvalue (Game|SpawnActorfromClass "/Game/BallGame/BP_TeleportTarget.BP_TeleportTarget_C" (Math|Transform|MakeTransform "0, 0, 0") "Undefined" 0 0))
  (Variables|Default|SetTargetActor _returnvalue))

(event EventTick
  (params (DeltaSeconds :type Float%20%28single-precision%29))
  (if (Variables|Default|GetBisTeleporting)
    (CallFunction|DetectHitpoint)))

(fn StartTeleporting
  (Variables|Default|SetBisTeleporting true)
  (Rendering|SetVisibility (Variables|/Game/BallGame/BP_TeleportTarget.BP_TeleportTarget_C|GetSphere (Variables|Default|GetTargetActor)) true false))

(fn EndTeleporting
  (bind _hitlocation (Variables|Default|GetHitLocation))
  (Variables|Default|SetBisTeleporting false)
  (if (Variables|Default|GetBhitsDetected)
    (Transformation|SetActorLocation (Variables|Default|GetActorToBeTeleported) (Math|Vector|MakeVector (.x _hitlocation) (.y _hitlocation) (+ (.z _hitlocation) 88.0)) false false)
    (Rendering|SetVisibility (Variables|/Game/BallGame/BP_TeleportTarget.BP_TeleportTarget_C|GetSphere (Variables|Default|GetTargetActor)) false false)))

(fn DetectHitpoint
  (bind _returnvalue (Transformation|GetWorldLocation))
  (bind _outhit (Collision|LineTraceByChannel _returnvalue (+ _returnvalue (* (Math|Vector|GetForwardVector) (Variables|Default|Getdistance))) "TraceTypeQuery1" false 0 "None"))
  (bind _output_get (Variables|Default|SetHitLocation (.location _outhit)))
  (bind _output_get_2 (Variables|Default|SetBhitsDetected (.bblockinghit _outhit)))
  (if _output_get_2
    (Transformation|SetActorLocation (Variables|Default|GetTargetActor) _output_get false false)))