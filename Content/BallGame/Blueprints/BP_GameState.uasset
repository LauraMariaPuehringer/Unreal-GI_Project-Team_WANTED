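; Game state for a ball game that tracks score, a countdown timer and the pool of inactive targets.
; On BeginPlay it gathers inactive BP_Target actors and activates one at random.
; AddPoints updates the score and starts the timer if it is stopped, so the countdown waits for the first score.
; Tick counts time down, broadcasts the remainder and calls GameFinished on the player controller at zero.
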(event EventBeginPlay
  (bind _returnvalue (Actor|GetActorOfClass "/Game/BallGame/Blueprints/BP_PlayerController.BP_PlayerController_C"))
  (Variables|Default|SetPlayerController _returnvalue)
  (CallFunction|SetUpTargets))

(event EventTick
  (params (DeltaSeconds :type Float%20%28single-precision%29))
  (if (Variables|Default|GettimerRunning)
    (Variables|Default|SettimeLeft (- (Variables|Default|GettimeLeft) DeltaSeconds))
    (Default|CallOnTimeLeftChanged (Variables|Default|GettimeLeft))
    (if (<= (Variables|Default|GettimeLeft) 0.0)
      (Variables|Default|SettimerRunning false)
      (Default|GameFinished (Variables|Default|GetPlayerController)))))

(fn ConstructionScript)

(fn AddPoints
  (params (Points :type Integer))
  (Utilities|FlowControl|Sequence
    (:then_0
      (Variables|Default|SetPoints (+ Points (Variables|Default|GetPoints)))
      (Default|CallOnPointsChanged (Variables|Default|GetPoints)))
    (:then_1
      (if (not (Variables|Default|GettimerRunning))
        (CallFunction|StartTimer)))))

(fn ActivateNext
  (bind _inactivetargets (Variables|Default|GetinactiveTargets))
  (if (> (Utilities|Array|Length _inactivetargets) 0)
    (Default|Activate (.OutItem (Utilities|Array|Random _inactivetargets)))))

(fn SetUpTargets
  (bind _inactivetargets (Variables|Default|GetinactiveTargets))
  (bind _outactors (Actor|GetAllActorsOfClass "/Game/BallGame/Blueprints/Target/BP_Target.BP_Target_C"))
  (Utilities|FlowControl|Sequence
    (:then_0
      (for _array_element _outactors
        (if (Variables|/Game/BallGame/Blueprints/Target/BP_Target.BP_Target_C|GetisActive _array_element)
          (Utilities|Array|RemoveItem _inactivetargets _array_element)
          (else
            (Utilities|Array|AddUnique _inactivetargets _array_element)))))
    (:then_1
      (CallFunction|ActivateNext))))

(fn StartTimer
  (Variables|Default|SetstartTime (Utilities|Time|GetGameTimeinSeconds))
  (Variables|Default|SettimerRunning true))