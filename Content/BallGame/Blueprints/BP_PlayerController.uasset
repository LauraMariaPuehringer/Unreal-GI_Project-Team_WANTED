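; BP_PlayerController is the ball game's player controller, handling the in-game menu and the game-finished state.
; The IngameMenu input flip-flops between PauseGame and ResumeGame through a gate.
; These toggle cursor, input mode, pawn input and the menu widget, without actually pausing game time.
; GameFinished shows the menu via PauseGame and closes the gate, so the input can no longer dismiss it.
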(event Custom|GameFinished
  (CallFunction|PauseGame)
  (Utilities|FlowControl|Gate false) ; enters at Close
)

(event Input|ActionEvents|InputActionIngameMenu
  (params (Key :type Key%20Structure :default "None"))
  (:Pressed
    (Utilities|FlowControl|Gate false
      (:Exit
        (Utilities|FlowControl|FlipFlop
          (:A
            (CallFunction|PauseGame))
          (:B
            (CallFunction|ResumeGame)))))))

(fn ConstructionScript)

(fn PauseGame
  (Variables|Default|SetbShowMouseCursor true)
  (Input|DisableInput (Game|Player|GetPlayerPawn 0) self)
  (Input|SetInputModeGameandUI self 0 "DoNotLock" false)
  (bind _returnvalue (UserInterface|CreateWidget "/Game/BallGame/Blueprints/WBP_IngameMenu.WBP_IngameMenu_C"))
  (bind _output_get (Variables|Default|SetIngameMenu _returnvalue))
  (UserInterface|Viewport|AddtoViewport _output_get 0))

(fn ResumeGame
  (Variables|Default|SetbShowMouseCursor false)
  (Input|EnableInput (Game|Player|GetPlayerPawn 0) self)
  (Input|SetInputModeGameOnly self)
  (Utilities|IsValid (Variables|Default|GetIngameMenu)
    (:Is%20Valid
      (Widget|RemovefromParent (Variables|Default|GetIngameMenu)))))