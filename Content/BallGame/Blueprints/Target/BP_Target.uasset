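; BP_Target is a ball-game target that awards points when hit while active and has a random number of hits, shown on its text.
; It starts red and inactive, and Activate turns it white.
; Each counted hit closes a three-second cooldown gate, adds a point through BP_GameState, calls SetUpTargets and decrements the counter.
; A dynamic material shows state, playing a color timeline after hits and turning purple on the last.
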(event OnComponentHit(Cube)
  (params (HitComponent :type Primitive%20Component%20Object%20Reference) (OtherActor :type Actor%20Object%20Reference) (OtherComp :type Primitive%20Component%20Object%20Reference) (NormalImpulse :type Vector :default "0, 0, 0") (Hit :type Hit%20Result%20Structure%20%28by%20ref%29))
  (if (Variables|Default|GetisActive)
    (if (> (Variables|Default|GethitsLeft) 0)
      (Utilities|FlowControl|Gate false :!label _label
        (:Exit
          (Rendering|Material|SetVectorParameterValue (Variables|Default|GetMaterial) "Color" "(R=0.000000,G=0.640625,B=0.000000,A=1.000000)" :!class /Script/Engine.MaterialInstanceDynamic)
          (Utilities|FlowControl|Sequence
            (:then_0
              (goto _label Close))
            (:then_1
              (if (<= (Variables|Default|GethitsLeft) 1)
                (Rendering|Material|SetVectorParameterValue (Variables|Default|GetMaterial) "Color" "(R=0.264679,G=0.034608,B=0.588542,A=1.000000)" :!class /Script/Engine.MaterialInstanceDynamic)
                (else
                  (bind _color (Timeline|ColorChange PlayFromStart)
                    (:Update
                      (Rendering|Material|SetVectorParameterValue (Variables|Default|GetMaterial) "Color" _color :!class /Script/Engine.MaterialInstanceDynamic))))))
            (:then_2
              (Utilities|FlowControl|Delay 3.0)
              (goto _label Open))
            (:then_3
              (Default|AddPoints (Variables|Default|GetGameState) 1))
            (:then_4
              (Default|SetUpTargets (Variables|Default|GetGameState)))
            (:then_5
              (bind _output_get (Variables|Default|SethitsLeft (- (Variables|Default|GethitsLeft) 1)))
              (Rendering|Components|TextRender|SetText (Variables|Default|GetTextRender) (Utilities|Text|ToText(Integer) _output_get)))))))))

(event EventBeginPlay
  (bind _returnvalue (Rendering|Material|CreateDynamicMaterialInstance (Variables|Default|GetCube) 0 "/Game/BallGame/Blueprints/Target/M_Target.M_Target" "None" :!class /Script/Engine.PrimitiveComponent))
  (Variables|Default|SetMaterial _returnvalue)
  (bind _asbp_game_state (Utilities|Casting|CastToBP_GameState (Game|GetGameState)))
  (Variables|Default|SetGameState _asbp_game_state)
  (Variables|Default|SetisActive false)
  (Rendering|Material|SetVectorParameterValue (Variables|Default|GetMaterial) "Color" (Class|KismetMathLibrary|LinearColorRed) :!class /Script/Engine.MaterialInstanceDynamic)
  (bind _output_get (Variables|Default|SethitsLeft (Math|Random|RandomIntegerinRange 5 10)))
  (Rendering|Components|TextRender|SetText (Variables|Default|GetTextRender) (Utilities|Text|ToText(Integer) _output_get)))

(fn ConstructionScript)

(fn Activate
  (Variables|Default|SetisActive true)
  (Rendering|Material|SetVectorParameterValue (Variables|Default|GetMaterial) "Color" "(R=1.000000,G=1.000000,B=1.000000,A=1.000000)" :!class /Script/Engine.MaterialInstanceDynamic))